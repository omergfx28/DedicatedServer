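; Networked player pawn that shows the player's name as floating 3D text.
; One second after BeginPlay, the locally controlled pawn sends its player name to the server, which sets the replicated PlayerName.
; Its RepNotify updates the text and tints the mesh with a locally randomized color, so colors are not synced between machines.
; On Tick, pawns not controlled by the local player turn their text toward the local camera.
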(event Custom|SetPlayerName%20%28Server%29
  (params (PlayerName :type String))
  ;[0 0 0] Oyuncu ismini sunucu üzerinde güncelle.
  (Variables|Default|SetPlayerName PlayerName))

(event EventBeginPlay
  ;[0 0 0] Begin play'de local da oyuncu ismini güncellemesi için sunucuya istek gönder.
  (Utilities|FlowControl|Delay 1.0)
  (if (Pawn|IsLocallyControlled)
    (CallFunction|SetPlayerName(Server) (Class|AdvancedSessionsLibrary|GetPlayerName (Game|GetPlayerController 0)))))

(event EventTick
  (params (DeltaSeconds :type Float%20%28single-precision%29))
  (bind _returnvalue (Game|GetPlayerController 0))
  (bind _textrender (Variables|Default|GetTextRender))
  ;[0 0 0] Rotasyonu güncelle.
  (if (!= (Pawn|GetController) _returnvalue)
    (Utilities|IsValid _textrender
      (:Is%20Valid
        (Transformation|SetWorldRotation _textrender (Math|Rotator|FindLookatRotation (Transformation|GetWorldLocation (Variables|Default|GetTextRender)) (Camera|GetCameraLocation (Variables|/Script/Engine.PlayerController|GetPlayerCameraManager _returnvalue))) false false)))))

(fn ConstructionScript)

(fn OnRepPlayerName
  (bind _textrender (Variables|Default|GetTextRender))
  (Utilities|IsValid _textrender
    (:Is%20Valid
      (Rendering|Components|TextRender|SetText _textrender (Utilities|Text|ToText(String) (Variables|Default|GetPlayerName)))
      (Rendering|Material|SetVectorParameterValueonMaterials (Variables|GetMeshComponent) "Color" (Math|Vector|MakeVector (Math|Random|RandomFloatinRange 0.0 1.0) (Math|Random|RandomFloatinRange 0.0 1.0) (Math|Random|RandomFloatinRange 0.0 1.0))))))